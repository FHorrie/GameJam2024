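; BP_Player is the player ship, carrying a machine gun and a speed-dependent trail effect.
; On BeginPlay it adds a BP_MachineGun component at the Arrow component's relative transform and stores it as Gun.
; Each tick it reads the capsule's physics linear velocity and toggles the NSShipTrail effect on or off around a speed threshold.
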(event `self.ReceiveBeginPlay`
  (`parent.ReceiveBeginPlay`)
  (bind _returnvalue (`|AddComponentByClass` "/Game/Blueprints/Character/Player/Guns/BP_MachineGun.BP_MachineGun_C" false (`SceneComponent.GetRelativeTransform` (`self.Arrow`))))
  (set `self.Gun` _returnvalue))

(event `self.ReceiveTick`
  (params (DeltaSeconds :type "Float (single-precision)"))
  (bind _ns_shiptrail (`self.NS_ShipTrail`))
  (`parent.ReceiveTick` DeltaSeconds)
  (bind _returnvalue (`PrimitiveComponent.GetPhysicsLinearVelocity` (`self.CapsuleComponent`) "None"))
  (if (>= (`KismetMathLibrary.VSize` _returnvalue) 100.0)
    (`ActorComponent.Activate` _ns_shiptrail false)
    (else
      (`ActorComponent.Deactivate` _ns_shiptrail))))

(fn `UserConstructionScript`
  (`parent.UserConstructionScript`))