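; BP_Sniper is a player gun Blueprint that defines the sniper's Fire function.
; Fire requires a BP_BaseCharacter owner and only shoots once accumulated shot time reaches the interval derived from the bullet RPM, then resets that timer.
; It spawns the bullet at a horizontal forward offset from the character, using the character's rotation and passing in owner speed, base damage and projectile speed.
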(fn `Fire`
  (locals (Offset :type "Float (double-precision)" :default 100.0))
  (bind _offset (`local.Offset`))
  (bind _asbp_base_character (cast `/Game/Blueprints/Character/BP_BaseCharacter` (`self.GetOwner`)))
  (if (>= (`self.AccuShotTime`) (/ 1.0 (/ (`self.BulletRPM`) 60.0)))
    (bind (_returnvalue_x _returnvalue_y _returnvalue_z) (`KismetMathLibrary.BreakVector` (`Actor.K2_GetActorLocation` _asbp_base_character)))
    (bind (_returnvalue_x_2 _returnvalue_y_2) (`KismetMathLibrary.BreakVector` (`Actor.GetActorForwardVector` _asbp_base_character)))
    (`|SpawnActorFromClass` (`self.Bullet`) (`KismetMathLibrary.MakeTransform` (`KismetMathLibrary.MakeVector` (+ _returnvalue_x (* _returnvalue_x_2 _offset)) (+ _returnvalue_y (* _returnvalue_y_2 _offset)) _returnvalue_z) (`Actor.K2_GetActorRotation` _asbp_base_character)) "AdjustIfPossibleButAlwaysSpawn" "MultiplyWithRoot" _asbp_base_character (`KismetMathLibrary.VSize` (`Actor.GetVelocity` _asbp_base_character)) 20.0 4000.0 null)
    (set `self.AccuShotTime` 0.0)))