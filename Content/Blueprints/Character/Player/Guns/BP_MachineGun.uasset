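; BP_MachineGun is a player weapon that fires bullets at a rate capped by its rounds-per-minute setting.
; Fire casts the owner to BP_Player and checks accumulated shot time against the interval derived from BulletRPM.
; When ready, it spawns a fixed-speed bullet offset horizontally along the player's forward vector, using the player's rotation, then resets the timer.
; Tick only calls the parent, and nothing here increments the timer.
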(event `self.ReceiveTick`
  (params (DeltaSeconds :type "Float (single-precision)"))
  (`parent.ReceiveTick` DeltaSeconds))

(fn `Fire`
  (locals (Bullet :type "/Game/Blueprints/Character/Player/Guns/Bullets/BP_BaseBullet Class Reference" :default "/Script/Engine.BlueprintGeneratedClass'/Game/Blueprints/Character/Player/Guns/Bullets/BP_MachineGunBullet.BP_MachineGunBullet_C'"))
  (bind _offset (`self.Offset`))
  (bind _asbp_player (cast `/Game/Blueprints/Character/Player/BP_Player` (`self.GetOwner`)))
  (if (>= (`self.AccuShotTime`) (/ 1.0 (/ (`self.BulletRPM`) 60.0)))
    (bind (_returnvalue_x _returnvalue_y _returnvalue_z) (`KismetMathLibrary.BreakVector` (`Actor.K2_GetActorLocation` _asbp_player)))
    (bind (_returnvalue_x_2 _returnvalue_y_2) (`KismetMathLibrary.BreakVector` (`Actor.GetActorForwardVector` _asbp_player)))
    (`|SpawnActorFromClass` (`local.Bullet`) (`KismetMathLibrary.MakeTransform` (`KismetMathLibrary.MakeVector` (+ _returnvalue_x (* _returnvalue_x_2 _offset)) (+ _returnvalue_y (* _returnvalue_y_2 _offset)) _returnvalue_z) (`Actor.K2_GetActorRotation` _asbp_player)) "AdjustIfPossibleButAlwaysSpawn" "MultiplyWithRoot" null 5.0 1300.0 null)
    (set `self.AccuShotTime` 0.0)))