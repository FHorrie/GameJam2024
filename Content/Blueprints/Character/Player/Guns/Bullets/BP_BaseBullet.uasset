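; BP_BaseBullet is a base projectile for player guns that flies along its forward vector in X and Y at a fixed height.
; Tick moves it manually while ShouldMove is set, and overlaps with other BP_BaseBullets are ignored.
; Overlapping a damageable actor while moving calls ProjectileHit, which applies point damage to its HitActor input (not supplied by the caller), stops movement and spawns Niagara impact effects.
; The bullet then destroys itself shortly afterward; non-damageable overlaps trigger delayed destruction without stopping it.
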(event `self.ReceiveActorBeginOverlap`
  (params (OtherActor :type "Actor Object Reference"))
  (cast `/Game/Blueprints/Character/Player/Guns/Bullets/BP_BaseBullet` OtherActor
    (:`CastFailed`
      (if (`Actor.bCanBeDamaged` OtherActor)
        (if (`self.ShouldMove`)
          (`self.ProjectileHit` null)
          (`KismetSystemLibrary.Delay` 0.2)
          (`self.K2_DestroyActor`))
        (else
          (`KismetSystemLibrary.Delay` 1.0)
          (`self.K2_DestroyActor`))))))

(event `self.ReceiveTick`
  (params (DeltaSeconds :type "Float (single-precision)"))
  (bind (_returnvalue_x _returnvalue_y) (`KismetMathLibrary.BreakVector` (`self.GetActorForwardVector`)))
  (bind (_returnvalue_x_2 _returnvalue_y_2 _returnvalue_z) (`KismetMathLibrary.BreakVector` (`self.K2_GetActorLocation`)))
  (bind _speed (`self.Speed`))
  (if (`self.ShouldMove`)
    (`self.K2_SetActorLocation` (`KismetMathLibrary.MakeVector` (+ (* DeltaSeconds (* _returnvalue_x _speed)) _returnvalue_x_2) (+ (* DeltaSeconds (* _returnvalue_y _speed)) _returnvalue_y_2) _returnvalue_z))))

(fn `ProjectileHit`
  (params (`Hit actor` :type "Actor Object Reference"))
  (`GameplayStatics.ApplyPointDamage` `Hit actor` (`self.BulletBaseDamage`) (`self.GetActorForwardVector`) (`GameplayStatics.MakeHitResult` false) null self "/Script/Engine.DamageType")
  (set `self.ShouldMove` false)
  (`NiagaraFunctionLibrary.SpawnSystemAtLocation` "/Game/Assets/FX/NS_BulletHit.NS_BulletHit" (`self.K2_GetActorLocation`) (`self.K2_GetActorRotation`)))

(fn `UserConstructionScript`)