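; BP_ShotGunBullet is a short-lived bullet for the player's shotgun.
; On BeginPlay, after the parent logic, it randomizes its speed and lifetime within narrow ranges, so each bullet differs in pace and reach.
; Tick runs the parent logic, accumulates time alive and destroys the actor once that lifetime is reached.
; It adds no movement or hit handling of its own, as its overlap event is a disabled stub.
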(event `self.ReceiveBeginPlay`
  (`parent.ReceiveBeginPlay`)
  (set `self.MaxAliveTime` (`KismetMathLibrary.RandomFloatInRange` 0.5 0.7))
  (set `self.Speed` (`KismetMathLibrary.RandomFloatInRange` 1000.0 1300.0)))

(event `self.ReceiveTick`
  (params (DeltaSeconds :type "Float (single-precision)"))
  (`parent.ReceiveTick` DeltaSeconds)
  (bind _output_get (set `self.AccuAliveTime` (+ DeltaSeconds (`self.AccuAliveTime`))))
  (if (>= _output_get (`self.MaxAliveTime`))
    (`self.K2_DestroyActor`)))

(fn `UserConstructionScript`
  (`parent.UserConstructionScript`))