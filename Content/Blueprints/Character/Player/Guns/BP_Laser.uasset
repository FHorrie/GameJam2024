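; Player laser gun that fires a continuous damaging beam along the owner's forward direction while toggling BP_Player's Laser component visibility.
; Fire and StopFire set the enabled state, and Tick runs a multi object trace that damages each damageable actor hit every frame, not scaled by delta time.
; Firing builds up accumulated time that drains at half rate when idle; reaching the limit forces a cooldown before it resets.
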(event `self.ReceiveBeginPlay`
  (bind _asbp_player (cast `/Game/Blueprints/Character/Player/BP_Player` (`self.GetOwner`)))
  (bind _laser (`/Game/Blueprints/Character/Player/BP_Player.Laser` _asbp_player))
  (`self.Activate` _laser false)
  (`self.SetHiddenInGame` _laser true false))

(event `self.ReceiveTick`
  (params (DeltaSeconds :type "Float (single-precision)"))
  (`parent.ReceiveTick` DeltaSeconds)
  (if (`self.LaserCooldown`)
    (`self.HandleCooldown` DeltaSeconds)
    (elif (`self.LaserEnabled`)
      (`self.UpdateLaser` DeltaSeconds)
      (else
        (`self.DecreaseAccuLaser` DeltaSeconds)))))

(event `UpdateLaser`
  (params (DeltaT :type "Float (double-precision)"))
  (bind _offset (`self.Offset`))
  (bind _laserdistance (`self.LaserDistance`))
  (set `self.LaserHitDistance` (`self.LaserDistance`))
  (bind _asbp_player (cast `/Game/Blueprints/Character/Player/BP_Player` (`self.GetOwner`)))
  (bind (_returnvalue_x _returnvalue_y _returnvalue_z) (`KismetMathLibrary.BreakVector` (`Actor.K2_GetActorLocation` _asbp_player)))
  (bind (_returnvalue_x_2 _returnvalue_y_2) (`KismetMathLibrary.BreakVector` (`Actor.GetActorForwardVector` _asbp_player)))
  (bind _outhits (`KismetSystemLibrary.LineTraceMultiForObjects` (`KismetMathLibrary.MakeVector` (+ _returnvalue_x (* _returnvalue_x_2 _offset)) (+ _returnvalue_y (* _returnvalue_y_2 _offset)) _returnvalue_z) (`KismetMathLibrary.MakeVector` (+ _returnvalue_x (* _returnvalue_x_2 _laserdistance)) (+ _returnvalue_y (* _returnvalue_y_2 _laserdistance)) _returnvalue_z) (`|MakeArray` "ObjectTypeQuery3" "ObjectTypeQuery2" :!type "EObjectTypeQuery Enum")))
  (for _array_element _outhits
    (bind (_bblockinghit _binitialoverlap _time _distance _location _impactpoint _normal _impactnormal _physmat _hitactor) (`GameplayStatics.BreakHitResult` _array_element))
    (`/Engine/EditorBlueprintResources/StandardMacros.IsValid` _hitactor
      (:`Is Valid`
        (if (`Actor.bCanBeDamaged` _hitactor)
          (`GameplayStatics.ApplyDamage` _hitactor 1.0)))
      (:`Is Not Valid`
        (set `self.LaserHitDistance` _distance)
        (break))))
  (bind _output_get (set `self.AccuLaserTIme` (+ (`self.AccuLaserTIme`) DeltaT)))
  (if (>= _output_get (`self.MaxLaserTime`))
    (set `self.LaserEnabled` false)
    (set `self.LaserCooldown` true)
    (bind _asbp_player_2 (cast `/Game/Blueprints/Character/Player/BP_Player` (`self.GetOwner`)))
    (`self.SetHiddenInGame` (`/Game/Blueprints/Character/Player/BP_Player.Laser` _asbp_player_2) true false)))

(event `DecreaseAccuLaser`
  (params (DeltaT :type "Float (double-precision)"))
  (if (> (`self.AccuLaserTIme`) 0.0)
    (set `self.AccuLaserTIme` (- (`self.AccuLaserTIme`) (/ DeltaT 2.0)))))

(event `HandleCooldown`
  (params (DeltaT :type "Float (double-precision)"))
  (bind _output_get (set `self.AccuCooldownTime` (+ (`self.AccuCooldownTime`) DeltaT)))
  (if (>= _output_get (`self.MaxCooldownTime`))
    (set `self.LaserCooldown` false)
    (set `self.AccuCooldownTime` 0.0)
    (set `self.AccuLaserTIme` 0.0)))

(fn `Fire`
  (if (`self.LaserEnabled`)
    _
    (elif (not (`self.LaserCooldown`))
      (set `self.LaserEnabled` true)
      (bind _asbp_player (cast `/Game/Blueprints/Character/Player/BP_Player` (`self.GetOwner`)))
      (`self.SetHiddenInGame` (`/Game/Blueprints/Character/Player/BP_Player.Laser` _asbp_player) false false))))

(fn `StopFire`
  (set `self.LaserEnabled` false)
  (bind _asbp_player (cast `/Game/Blueprints/Character/Player/BP_Player` (`self.GetOwner`)))
  (`self.SetHiddenInGame` (`/Game/Blueprints/Character/Player/BP_Player.Laser` _asbp_player) true false))