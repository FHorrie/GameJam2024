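; BP_ShotGun is a player gun Blueprint that fires a spread of pellets from its owning BP_Player.
; Fire is gated by accumulated shot time against a rate derived from BulletRPM, then resets that timer.
; A loop spawns BulletType actors at a horizontal offset ahead of the player, each with random yaw within a narrow cone around the player's rotation.
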(fn `Fire`
  (locals (BulletType :type "/Game/Blueprints/Character/Player/Guns/Bullets/BP_BaseBullet Class Reference" :default "/Script/Engine.BlueprintGeneratedClass'/Game/Blueprints/Character/Player/Guns/Bullets/BP_ShotGunBullet.BP_ShotGunBullet_C'") (AmountOfPellets :type Integer :default 25) (Offset :type "Float (double-precision)" :default 100.0))
  (bind _offset (`local.Offset`))
  (bind _asbp_player (cast `/Game/Blueprints/Character/Player/BP_Player` (`self.GetOwner`)))
  (if (>= (`self.AccuShotTime`) (/ 1.0 (/ (`self.BulletRPM`) 60.0)))
    (for _ (range (+ (`local.AmountOfPellets`) 1))
      (bind (_returnvalue_x _returnvalue_y _returnvalue_z) (`KismetMathLibrary.BreakVector` (`Actor.K2_GetActorLocation` _asbp_player)))
      (bind (_returnvalue_x_2 _returnvalue_y_2) (`KismetMathLibrary.BreakVector` (`Actor.GetActorForwardVector` _asbp_player)))
      (`|SpawnActorFromClass` (`local.BulletType`) (`KismetMathLibrary.MakeTransform` (`KismetMathLibrary.MakeVector` (+ _returnvalue_x (* _returnvalue_x_2 _offset)) (+ _returnvalue_y (* _returnvalue_y_2 _offset)) _returnvalue_z) (`KismetMathLibrary.ComposeRotators` (`Actor.K2_GetActorRotation` _asbp_player) (`KismetMathLibrary.MakeRotator` 0.0 0.0 (`KismetMathLibrary.RandomFloatInRange` -10.0 10.0)))) "AdjustIfPossibleButAlwaysSpawn" "MultiplyWithRoot" null 5.0 1300.0 null))
    (set `self.AccuShotTime` 0.0)))