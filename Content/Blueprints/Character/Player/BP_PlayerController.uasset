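; Player controller that turns Enhanced Input actions into rotation, thrust, firing and pause for BP_Player.
; Rotate input accumulates a desired yaw, which Tick smoothly lerps into the control rotation.
; Move pushes along the pawn's forward vector and toggles engine state and plasma audio, fire drives the pawn's gun, and pause toggles the HUD menu.
; A cursor-trace LookAtMouse function is defined but not called here.
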(event `self.ReceiveBeginPlay`
  (bind _returnvalue (subsystem `EnhancedInputLocalPlayerSubsystem`))
  (`/Engine/EditorBlueprintResources/StandardMacros.IsValid` _returnvalue
    (:`Is Valid`
      (`EnhancedInputSubsystemInterface.AddMappingContext` _returnvalue "/Game/Blueprints/Input/IMC_PlayerInput.IMC_PlayerInput" 0 (struct)))))

(event `self.ReceiveTick`
  (params (DeltaSeconds :type "Float (single-precision)"))
  (`self.LerpRotation` DeltaSeconds))

(event `EnhancedInput|/Game/Blueprints/Input/Controls/IA_Rotate`
  (params (ActionValue :type "Float (double-precision)") (ElapsedSeconds :type "Float (double-precision)") (TriggeredSeconds :type "Float (double-precision)") (InputAction :type "InputAction Object Reference" :default "/Game/Blueprints/Input/Controls/IA_Rotate.IA_Rotate"))
  (:`Triggered`
    (`self.AddDesiredRotation` (* (`self.RotationSpeed`) ActionValue))))

(event `EnhancedInput|/Game/Blueprints/Input/Controls/IA_Fire`
  (params (ActionValue :type Boolean) (ElapsedSeconds :type "Float (double-precision)") (TriggeredSeconds :type "Float (double-precision)") (InputAction :type "InputAction Object Reference" :default "/Game/Blueprints/Input/Controls/IA_Fire.IA_Fire"))
  (:`Triggered`
    (bind _asbp_player (cast `/Game/Blueprints/Character/Player/BP_Player` (`self.K2_GetPawn`)))
    (`/Game/Blueprints/Character/Player/Guns/BP_BaseWeapon.Fire` (`/Game/Blueprints/Character/Player/BP_Player.Gun` _asbp_player)))
  (:`Completed`
    (bind _asbp_player_2 (cast `/Game/Blueprints/Character/Player/BP_Player` (`self.K2_GetPawn`)))
    (`/Game/Blueprints/Character/Player/Guns/BP_BaseWeapon.StopFire` (`/Game/Blueprints/Character/Player/BP_Player.Gun` _asbp_player_2))))

(event `EnhancedInput|/Game/Blueprints/Input/Controls/IA_Move`
  (params (ActionValue :type "Float (double-precision)") (ElapsedSeconds :type "Float (double-precision)") (TriggeredSeconds :type "Float (double-precision)") (InputAction :type "InputAction Object Reference" :default "/Game/Blueprints/Input/Controls/IA_Move.IA_Move"))
  (bind _returnvalue (`self.K2_GetPawn`))
  (:`Triggered`
    (`Pawn.AddMovementInput` _returnvalue (* (`self.GetActorForwardVector` _returnvalue) ActionValue) 1.0 false))
  (:`Started`
    (bind _asbp_player (cast `/Game/Blueprints/Character/Player/BP_Player` _returnvalue))
    (`/Game/Blueprints/Character/Player/BP_Player.EngineOn` _asbp_player)
    (`AudioComponent.Play` (`/Game/Blueprints/Character/BP_BaseCharacter.plasma-engine-fx-33559` _asbp_player) 0.0))
  (:`Completed`
    (bind _asbp_player_2 (cast `/Game/Blueprints/Character/Player/BP_Player` _returnvalue))
    (`/Game/Blueprints/Character/Player/BP_Player.EngineOff` _asbp_player_2)
    (`AudioComponent.Stop` (`/Game/Blueprints/Character/BP_BaseCharacter.plasma-engine-fx-33559` _asbp_player_2))))

(event `EnhancedInput|/Game/Blueprints/Input/Controls/IA_Pause`
  (params (ActionValue :type Boolean) (ElapsedSeconds :type "Float (double-precision)") (TriggeredSeconds :type "Float (double-precision)") (InputAction :type "InputAction Object Reference" :default "/Game/Blueprints/Input/Controls/IA_Pause.IA_Pause"))
  (:`Started`
    (bind _asbp_player_hud (cast `/Game/Blueprints/UI/BP_PlayerHUD` (`self.GetHUD`)))
    (`/Game/Blueprints/UI/BP_PlayerHUD.TogglePauseMenu` _asbp_player_hud)))

(fn `AddDesiredRotation`
  (params (Angle :type "Float (double-precision)"))
  (bind (_desiredrotation_roll _desiredrotation_pitch _desiredrotation_yaw) (`KismetMathLibrary.BreakRotator` (`self.DesiredRotation`)))
  (set `self.DesiredRotation` (`KismetMathLibrary.MakeRotator` _desiredrotation_roll _desiredrotation_pitch (+ _desiredrotation_yaw Angle))))

(fn `LerpRotation`
  (params (DeltaTime :type "Float (double-precision)"))
  (`self.SetControlRotation` (`KismetMathLibrary.RLerp` (`self.GetDesiredRotation`) (`self.DesiredRotation`) (* DeltaTime (`self.LerpIntensity`)) true)))

(fn `LookAtMouse`
  (params (DeltaTime :type "Float (double-precision)"))
  (bind (_worldlocation _worlddirection) (`self.DeprojectMousePositionToWorld`))
  (bind _outhit (`KismetSystemLibrary.LineTraceSingle` _worldlocation (+ _worldlocation (* _worlddirection 10000.0)) "TraceTypeQuery1"))
  (`self.SetControlRotation` (`KismetMathLibrary.RLerp` (`self.GetDesiredRotation`) (`KismetMathLibrary.MakeRotFromX` (- (`.Location` (`GameplayStatics.BreakHitResult` _outhit)) (`self.K2_GetActorLocation` (`self.K2_GetPawn`)))) (* DeltaTime (`self.LerpIntensity`)) true)))

(fn `UserConstructionScript`)