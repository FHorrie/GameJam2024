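; Base character pawn using FloatingPawnMovement, with an IsDead health check and a filter for abrupt velocity changes.
; Each Tick, BigVelocityChange compares squared 2D velocity difference against a max-speed-based threshold; its dot-product check follows an unconditional return.
; On a big change, Tick pauses OldVelocity tracking, then restores that saved velocity after a short Delay.
; Current velocity prints every frame for debugging.
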(event `self.ReceiveTick`
  (params (DeltaSeconds :type "Float (single-precision)"))
  (`|ExecutionSequence`
    (:`then_0`
      (if (`self.BigVelocityChange`)
        (set `self.RecentlyChanged` true)
        (`KismetSystemLibrary.Delay` 0.05)
        (set `MovementComponent.Velocity` (`self.OldVelocity`) (`self.FloatingPawnMovement`))
        (set `self.RecentlyChanged` false)))
    (:`then_1`
      (if (not (`self.RecentlyChanged`))
        (set `self.OldVelocity` (`self.GetVelocity`))))
    (:`then_2`
      (`KismetSystemLibrary.PrintString` (`KismetStringLibrary.Conv_VectorToString` (`self.GetVelocity`)) true true (struct :`G` 0.66 :`B` 1.0 :`A` 1.0) 2.0 "5"))))

(fn `BigVelocityChange`
  (returns (Changed :type Boolean))
  (`|ExecutionSequence`
    (:`then_0`
      (return (> (`KismetMathLibrary.Vector_Distance2DSquared` (`self.OldVelocity`) (`self.GetVelocity`)) (* (`KismetMathLibrary.MultiplyMultiply_FloatFloat` (`MovementComponent.GetMaxSpeed` (`self.FloatingPawnMovement`)) 2.0) 2.0))))
    (:`then_1`
      (return (< (`KismetMathLibrary.Dot_VectorVector` (`self.OldVelocity`) (`self.GetVelocity`)) 0.5)))))

(fn `IsDead`
  (returns (Dead :type Boolean))
  (return (< (`self.Health`) 0.0)))

(fn `UserConstructionScript`)