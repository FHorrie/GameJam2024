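; BP_BaseEnemy is a base enemy Blueprint that feeds the player's position to its AI and handles death.
; Every Tick it writes the location of player pawn 0 into the PlayerPos Blackboard key.
; Its Die override calls the parent version, spawns a water-ball hit particle effect at the actor's transform, then destroys the actor.
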(event `self.ReceiveTick`
  (params (DeltaSeconds :type "Float (single-precision)"))
  (`BlackboardComponent.SetValueAsVector` (`AIBlueprintHelperLibrary.GetBlackboard` null) (`self.PlayerPos`) (`self.K2_GetActorLocation` (`GameplayStatics.GetPlayerPawn` 0))))

(fn `Die`
  (bind (_returnvalue_location _returnvalue_rotation _returnvalue_scale) (`KismetMathLibrary.BreakTransform` (`self.GetTransform`)))
  (`parent.Die`)
  (`GameplayStatics.SpawnEmitterAtLocation` "/Game/FXVarietyPack/Particles/P_ky_waterBallHit.P_ky_waterBallHit" _returnvalue_location _returnvalue_rotation _returnvalue_scale)
  (`self.K2_DestroyActor`))

(fn `UserConstructionScript`
  (`parent.UserConstructionScript`))