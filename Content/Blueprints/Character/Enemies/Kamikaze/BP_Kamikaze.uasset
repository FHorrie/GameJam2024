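; BP_Kamikaze is an enemy character that destroys itself on contact with a damageable actor.
; Every tick it writes the player pawn's location to the PlayerPos blackboard key, presumably for its AI to chase.
; When its collision box overlaps an actor that can be damaged, it spawns a water-ball hit particle at its own transform and destroys itself.
; The graph itself applies no damage.
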(event `self.ReceiveTick`
  (params (DeltaSeconds :type "Float (single-precision)"))
  (`BlackboardComponent.SetValueAsVector` (`AIBlueprintHelperLibrary.GetBlackboard` null) (`self.PlayerPos`) (`self.K2_GetActorLocation` (`GameplayStatics.GetPlayerPawn` 0))))

(event `self.CollisionBox.OnComponentBeginOverlap`
  (params (OverlappedComponent :type "PrimitiveComponent Object Reference") (OtherActor :type "Actor Object Reference") (OtherComp :type "PrimitiveComponent Object Reference") (OtherBodyIndex :type Integer) (bFromSweep :type Boolean) (SweepResult :type "HitResult Structure (by ref)"))
  (bind (_returnvalue_location _returnvalue_rotation _returnvalue_scale) (`KismetMathLibrary.BreakTransform` (`self.GetTransform`)))
  (if (`Actor.bCanBeDamaged` OtherActor)
    (`GameplayStatics.SpawnEmitterAtLocation` "/Game/FXVarietyPack/Particles/P_ky_waterBallHit.P_ky_waterBallHit" _returnvalue_location _returnvalue_rotation _returnvalue_scale)
    (`self.K2_DestroyActor`)))

(fn `UserConstructionScript`
  (`parent.UserConstructionScript`))