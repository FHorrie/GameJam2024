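; BP_GunnerController is the AI controller for the Gunner enemy, deciding when it retreats from or can fire at the player.
; Each Tick it measures the distance between its controlled pawn and player pawn 0.
; It sets the ShouldRetreat Blackboard flag inside the minimum move-back range, and CanFire between that range and maximum fire range.
; The checks use distance alone, with no line-of-sight test.
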(event `self.ReceiveTick`
  (params (DeltaSeconds :type "Float (single-precision)"))
  (bind _blackboard (`self.Blackboard`))
  (bind _shouldretreat (`self.ShouldRetreat`))
  (bind _canfire (`self.CanFire`))
  (bind _returnvalue (`KismetMathLibrary.VSize` (- (`self.K2_GetActorLocation` (`GameplayStatics.GetPlayerPawn` 0)) (`self.K2_GetActorLocation` (`self.K2_GetPawn`)))))
  (bind _returnvalue_2 (< _returnvalue (`self.MinMoveBackRange`)))
  (`|ExecutionSequence`
    (:`then_0`
      (if _returnvalue_2
        (`BlackboardComponent.SetValueAsBool` _blackboard _shouldretreat true)
        (else
          (`BlackboardComponent.SetValueAsBool` _blackboard _shouldretreat false))))
    (:`then_1`
      (if (and (not _returnvalue_2) (< _returnvalue (`self.MaxFireRange`)))
        (`BlackboardComponent.SetValueAsBool` _blackboard _canfire true)
        (else
          (`BlackboardComponent.SetValueAsBool` _blackboard _canfire false))))))

(fn `UserConstructionScript`
  (`parent.UserConstructionScript`))