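; Gunner enemy character that equips itself with a sniper weapon firing enemy bullets.
; On BeginPlay it runs the parent logic, adds a BP_Sniper component at Arrow1's relative transform and stores it as Gun.
; It hides the gun in game without propagating to children, then sets its bullet to BP_SniperBulletEnemy.
; Tick and construction only call the parent, so this file holds no firing logic.
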(event `self.ReceiveBeginPlay`
  (`parent.ReceiveBeginPlay`)
  (bind _returnvalue (`|AddComponentByClass` "/Game/Blueprints/Character/Player/Guns/BP_Sniper.BP_Sniper_C" false (`SceneComponent.GetRelativeTransform` (`self.Arrow1`))))
  (bind _output_get (set `self.Gun` _returnvalue))
  (`SceneComponent.SetHiddenInGame` _output_get true false)
  (set `/Game/Blueprints/Character/Player/Guns/BP_Sniper.Bullet` "/Game/Blueprints/Character/Player/Guns/Bullets/BP_SniperBulletEnemy.BP_SniperBulletEnemy_C" _returnvalue))

(event `self.ReceiveTick`
  (params (DeltaSeconds :type "Float (single-precision)"))
  (`parent.ReceiveTick` DeltaSeconds))

(fn `UserConstructionScript`
  (`parent.UserConstructionScript`))