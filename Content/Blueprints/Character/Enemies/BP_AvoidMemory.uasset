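; BP_AvoidMemory is a component on the enemy AI controller that steers its BP_BaseEnemy pawn using remembered teammates.
; It keeps a Teammates list, maintained through add and remove functions.
; Each Tick it adds their velocities to a persistent NewDirection, normalizes it and adds that to the pawn's FloatingPawnMovement velocity.
; Despite the name, this aligns movement with teammates, like flocking alignment, with no distance or repulsion term.
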(event `self.ReceiveTick`
  (params (DeltaSeconds :type "Float (single-precision)"))
  (if (`KismetArrayLibrary.Array_IsNotEmpty` (`self.Teammates`))
    (for _array_element (`self.Teammates`)
      (set `self.NewDirection` (+ (`Actor.GetVelocity` _array_element) (`self.NewDirection`))))
    (set `self.NewDirection` (`KismetMathLibrary.Normal` (`self.NewDirection`)))
    (bind _asbp_base_enemy_controlller (cast `/Game/Blueprints/Character/Enemies/BP_BaseEnemyControlller` (`self.GetOwner`)))
    (bind _asbp_base_enemy (cast `/Game/Blueprints/Character/Enemies/BP_BaseEnemy` (`Controller.K2_GetPawn` _asbp_base_enemy_controlller)))
    (bind _floatingpawnmovement (`/Game/Blueprints/Character/BP_BaseCharacter.FloatingPawnMovement` _asbp_base_enemy))
    (set `MovementComponent.Velocity` (+ (`MovementComponent.Velocity` _floatingpawnmovement) (`self.NewDirection`)) _floatingpawnmovement)))

(fn `AddTeammate`
  (params (Teammate :type "/Game/Blueprints/Character/Enemies/BP_BaseEnemy Object Reference"))
  (`KismetArrayLibrary.Array_Add` (`self.Teammates`) Teammate))

(fn `RemoveTeammate`
  (params (Teammate :type "/Game/Blueprints/Character/Enemies/BP_BaseEnemy Object Reference"))
  (`KismetArrayLibrary.Array_RemoveItem` (`self.Teammates`) Teammate))