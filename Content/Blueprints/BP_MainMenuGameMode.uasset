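; Game mode for the main menu that creates and manages the main menu and credits widgets.
; On BeginPlay it adds both widgets to the viewport with credits collapsed, shows the mouse cursor and sets UI-only input focused on the menu, locking the mouse in fullscreen.
; A ToggleCredits event swaps visibility between the two widgets, tracking the state with a boolean.
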(event `self.ReceiveBeginPlay`
  (bind _returnvalue (`GameplayStatics.GetPlayerController` 0))
  (bind _returnvalue_2 (`|GenericCreateObject` "/Game/Blueprints/UI/WBP_MainMenu.WBP_MainMenu_C"))
  (bind _output_get (set `self.MainMenuRef` _returnvalue_2))
  (`UserWidget.AddToViewport` _output_get 0)
  (set `PlayerController.bShowMouseCursor` true _returnvalue)
  (`WidgetBlueprintLibrary.SetInputMode_UIOnlyEx` _returnvalue (`self.MainMenuRef`) "LockInFullscreen")
  (bind _returnvalue_3 (`|GenericCreateObject` "/Game/Blueprints/UI/WBP_Credits.WBP_Credits_C"))
  (bind _output_get_2 (set `self.CreditsRef` _returnvalue_3))
  (`UserWidget.AddToViewport` _output_get_2 0)
  (`Widget.SetVisibility` _output_get_2 "Collapsed"))

(event `ToggleCredits`
  (if (`self.AreCreditsVisible`)
    (`Widget.SetVisibility` (`self.CreditsRef`) "Collapsed")
    (`Widget.SetVisibility` (`self.MainMenuRef`) "Visible")
    (set `self.AreCreditsVisible` false)
    (else
      (`Widget.SetVisibility` (`self.CreditsRef`) "Visible")
      (`Widget.SetVisibility` (`self.MainMenuRef`) "Collapsed")
      (set `self.AreCreditsVisible` true))))

(fn `UserConstructionScript`)