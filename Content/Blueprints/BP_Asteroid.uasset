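; Asteroid actor that drifts at a set direction and speed, deals environmental damage on overlap, and breaks apart when shot.
; Construction scales its damage by average actor scale, and Tick moves it without sweeping.
; Point damage destroys it after SplitAsteroid spawns smaller pieces at mirrored yaw angles around a vector blending travel and reversed shot direction.
; An AllowSplit minimum-size check is defined but never called.
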(event `self.ReceiveBeginPlay`
  (add `self.OnTakePointDamage` (delegate `OnTakePointDamage_Event`)))

(event `OnTakePointDamage_Event` :!signature `self.OnTakePointDamage`
  (params (DamagedActor :type "Actor Object Reference") (Damage :type "Float (single-precision)") (InstigatedBy :type "Controller Object Reference") (HitLocation :type "Vector Structure") (FHitComponent :type "PrimitiveComponent Object Reference") (BoneName :type Name) (ShotFromDirection :type "Vector Structure") (DamageType :type "DamageType Object Reference") (DamageCauser :type "Actor Object Reference"))
  (`self.SplitAsteroid` 2 45.0 ShotFromDirection)
  (`self.K2_DestroyActor`))

(event `self.ReceiveActorBeginOverlap`
  (params (OtherActor :type "Actor Object Reference"))
  (`self.Hit` OtherActor))

(event `self.ReceiveTick`
  (params (DeltaSeconds :type "Float (single-precision)"))
  (`self.UpdateLocation` DeltaSeconds))

(fn `AllowSplit`
  (returns (AllowSplit :type Boolean))
  (return (> (`self.GetAverageScale`) 0.2)))

(fn `GetAverageScale`
  (returns (AverageScale :type "Float (double-precision)"))
  (bind (_returnvalue_x _returnvalue_y _returnvalue_z) (`KismetMathLibrary.BreakVector` (`self.GetActorScale3D`)))
  (return (/ (+ _returnvalue_x _returnvalue_y _returnvalue_z) 3.0)))

(fn `Hit`
  (params (`Hit Actor` :type "Actor Object Reference"))
  (`GameplayStatics.ApplyPointDamage` null (`self.InstanceDamage`) (- (`self.K2_GetActorLocation` `Hit Actor`) (`self.K2_GetActorLocation` self)) (`GameplayStatics.MakeHitResult` false true) null self "/Engine/EngineDamageTypes/DmgTypeBP_Environmental.DmgTypeBP_Environmental_C"))

(fn `SplitAsteroid`
  (params (NumberOfPieces :type Integer) (RangeOnSide :type "Float (double-precision)") (ShotDirection :type "Vector Structure"))
  (locals (AnglePerPiece :type "Float (double-precision)") (NrOfPiecesPerSide :type Integer) (HalfVector :type "Vector Structure") (PieceScale :type "Vector Structure"))
  (`|ExecutionSequence`
    (:`then_0`
      ;[1 1 1] Setup variables
      ;;[1 1 1] Get half vector
      (set `local.HalfVector` (`KismetMathLibrary.Normal` (/ (+ (`self.Direction`) (* ShotDirection -1.0)) 2.0)))
      ;;[1 1 1] Get Nr of pieces on each side
      (bind _output_get (set `local.NrOfPiecesPerSide` (/ NumberOfPieces 2)))
      ;;[1 1 1] Get incremental angle each piece launches
      (set `local.AnglePerPiece` (/ RangeOnSide _output_get))
      ;;[1 1 1] Scale of smaller pieces
      (set `local.PieceScale` (/ (`self.GetActorScale3D`) NumberOfPieces)))
    (:`then_1`
      ;[1 1 1] Split pieces
      (bind _result (`/Engine/EditorBlueprintResources/StandardMacros.IncrementInt` (`local.NrOfPiecesPerSide`))
        (:`  `
          (for _index (range 1 (+ _result 1))
            (`|ExecutionSequence`
              (:`then_0`
                (bind _returnvalue (* _index (`local.AnglePerPiece`)))
                (bind _returnvalue_2 (`KismetMathLibrary.GreaterGreater_VectorRotator` (`local.HalfVector`) (`KismetMathLibrary.MakeRotator` 0.0 0.0 _returnvalue)))
                ;;[1 1 1] Spawn piece to left of direction
                (`|SpawnActorFromClass` "BP_Asteroid_C" (`KismetMathLibrary.MakeTransform` (`self.K2_GetActorLocation`) (`KismetMathLibrary.Conv_VectorToRotator` _returnvalue_2) (`local.PieceScale`)) "AdjustIfPossibleButAlwaysSpawn" "MultiplyWithRoot" null _returnvalue_2 (`self.Speed`) null))
              (:`then_1`
                (bind _returnvalue_3 (`KismetMathLibrary.GreaterGreater_VectorRotator` (`local.HalfVector`) (`KismetMathLibrary.MakeRotator` 0.0 0.0 (* _returnvalue -1.0))))
                ;;[1 1 1] Spawn piece to right of direction
                (`|SpawnActorFromClass` "BP_Asteroid_C" (`KismetMathLibrary.MakeTransform` (`self.K2_GetActorLocation`) (`KismetMathLibrary.Conv_VectorToRotator` _returnvalue_3) (`local.PieceScale`)) "AdjustIfPossibleButAlwaysSpawn" "MultiplyWithRoot" null _returnvalue_3 (`self.Speed`) null)))))))))

(fn `UpdateLocation`
  (params (DeltaTime :type "Float (double-precision)"))
  (`self.K2_AddActorWorldOffset` (* DeltaTime (* (`self.Direction`) (`self.Speed`)))))

(fn `UserConstructionScript`
  (set `self.InstanceDamage` (* (`self.GetAverageScale`) (`self.BaseDamage`))))