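; BP_Asteroid is an asteroid that splits into smaller asteroids when damaged, as long as its average scale exceeds MinScale.
; TakeDamage checks AllowSplit, then passes the shot direction to SplitAsteroid.
; SplitAsteroid derives a flattened half vector from its travel direction and the negated shot direction.
; It spawns scaled-down pieces in mirrored yaw steps around that vector, each keeping the parent's speed.
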(fn `AllowSplit`
  (returns (AllowSplit :type Boolean))
  (locals (MinScale :type "Float (double-precision)" :default 0.2))
  (return (> (`self.GetAverageScale`) (`local.MinScale`))))

(fn `SplitAsteroid`
  (params (NumberOfPieces :type Integer) (RangeOnSide :type "Float (double-precision)") (ShotDirection :type "Vector Structure"))
  (locals (AnglePerPiece :type "Float (double-precision)") (NrOfPiecesPerSide :type Integer) (HalfVector :type "Vector Structure") (PieceScale :type "Vector Structure"))
  (bind (_returnvalue_x _returnvalue_y) (`KismetMathLibrary.BreakVector` (+ (`self.Direction`) (* ShotDirection -1.0))))
  (`|ExecutionSequence`
    (:`then_0`
      ;[1 1 1] Setup variables
      ;;[1 1 1] Get half vector
      (set `local.HalfVector` (`KismetMathLibrary.Normal` (`KismetMathLibrary.MakeVector` (* _returnvalue_x 0.5) (* _returnvalue_y 0.5))))
      ;;[1 1 1] Get Nr of pieces on each side
      (bind _output_get (set `local.NrOfPiecesPerSide` (/ NumberOfPieces 2)))
      ;;[1 1 1] Get incremental angle each piece launches
      (set `local.AnglePerPiece` (/ RangeOnSide _output_get))
      ;;[1 1 1] Scale of smaller pieces
      (set `local.PieceScale` (/ (`self.GetActorScale3D`) NumberOfPieces)))
    (:`then_1`
      ;[1 1 1] Split pieces
      (bind _result (`/Engine/EditorBlueprintResources/StandardMacros.IncrementInt` (`local.NrOfPiecesPerSide`))
        (:`  `
          (for _index (range 1 (+ _result 1))
            (`|ExecutionSequence`
              (:`then_0`
                (bind _returnvalue (* _index (`local.AnglePerPiece`)))
                (bind _returnvalue_2 (`KismetMathLibrary.GreaterGreater_VectorRotator` (`local.HalfVector`) (`KismetMathLibrary.MakeRotator` 0.0 0.0 _returnvalue)))
                ;;[1 1 1] Spawn piece to left of direction
                (`|SpawnActorFromClass` "BP_Asteroid_C" (`KismetMathLibrary.MakeTransform` (`self.K2_GetActorLocation`) (`KismetMathLibrary.Conv_VectorToRotator` _returnvalue_2) (`local.PieceScale`)) "AdjustIfPossibleButAlwaysSpawn" "MultiplyWithRoot" null _returnvalue_2 (`self.Speed`) null))
              (:`then_1`
                (bind _returnvalue_3 (`KismetMathLibrary.GreaterGreater_VectorRotator` (`local.HalfVector`) (`KismetMathLibrary.MakeRotator` 0.0 0.0 (* _returnvalue -1.0))))
                ;;[1 1 1] Spawn piece to right of direction
                (`|SpawnActorFromClass` "BP_Asteroid_C" (`KismetMathLibrary.MakeTransform` (`self.K2_GetActorLocation`) (`KismetMathLibrary.Conv_VectorToRotator` _returnvalue_3) (`local.PieceScale`)) "AdjustIfPossibleButAlwaysSpawn" "MultiplyWithRoot" null _returnvalue_3 (`self.Speed`) null)))))))))

(fn `TakeDamage`
  (params (ShotFromDirection :type "Vector Structure") (DamageType :type "DamageType Object Reference") (DamageCauser :type "Actor Object Reference"))
  (if (`self.AllowSplit`)
    (`self.SplitAsteroid` 2 45.0 ShotFromDirection)))

(fn `UserConstructionScript`
  (`parent.UserConstructionScript`))