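; BP_DebrisSpawner is an environment spawner that creates a debris actor at its own location each time its Spawn event runs.
; Each spawn receives a random scale and speed within configured min/max ranges, plus a random direction for movement and facing.
; Two arrow components define the direction cone, centered between their forward vectors and spanning the angle between them, with Z zeroed to keep directions horizontal.
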(event `self.Spawn`
  (bind _direction (`self.RandomDirection`))
  (`|SpawnActorFromClass` (`self.DebrisClass`) (`KismetMathLibrary.MakeTransform` (`self.K2_GetActorLocation`) (`KismetMathLibrary.MakeRotFromX` _direction) (`self.RandomScale`)) "Undefined" "MultiplyWithRoot" null _direction (`self.RandomSpeed`) null))

(fn `RandomDirection`
  (returns (Direction :type "Vector Structure"))
  (bind _returnvalue (`SceneComponent.GetForwardVector` (`self.RangeArrowLeft`)))
  (bind _returnvalue_2 (`SceneComponent.GetForwardVector` (`self.RangeArrowRight`)))
  (bind (_returnvalue_x _returnvalue_y) (`KismetMathLibrary.BreakVector` (`KismetMathLibrary.RandomUnitVectorInConeInDegrees` (* (+ _returnvalue _returnvalue_2) 0.5) (* (`KismetMathLibrary.DegAcos` (`KismetMathLibrary.Dot_VectorVector` _returnvalue _returnvalue_2)) 0.5))))
  (return (`KismetMathLibrary.MakeVector` _returnvalue_x _returnvalue_y)))

(fn `RandomScale`
  (returns (Scale :type "Vector Structure"))
  (bind (_minscale_x _minscale_y _minscale_z) (`KismetMathLibrary.BreakVector` (`self.MinScale`)))
  (bind (_maxscale_x _maxscale_y _maxscale_z) (`KismetMathLibrary.BreakVector` (`self.MaxScale`)))
  (return (`KismetMathLibrary.MakeVector` (`KismetMathLibrary.RandomFloatInRange` _minscale_x _maxscale_x) (`KismetMathLibrary.RandomFloatInRange` _minscale_y _maxscale_y) (`KismetMathLibrary.RandomFloatInRange` _minscale_z _maxscale_z))))

(fn `RandomSpeed`
  (returns (Speed :type "Float (double-precision)"))
  (return (`KismetMathLibrary.RandomFloatInRange` (`self.MinSpeed`) (`self.MaxSpeed`))))

(fn `UserConstructionScript`
  (`parent.UserConstructionScript`))