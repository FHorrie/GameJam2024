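; BP_PickUpSpawner is an environment actor that spawns a random pickup somewhere inside a configurable box zone.
; Its construction script sizes the SpawnZone box from half the ZoneHeight on X and half the ZoneWidth on Y, with a fixed Z extent.
; The Spawn event picks a random class from PossiblePickUps and places it at a random point around the actor, within the box's scaled X/Y extents.
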(event `self.Spawn`
  (`|SpawnActorFromClass` (`KismetArrayLibrary.Array_Random` (`self.PossiblePickUps`)) (`KismetMathLibrary.MakeTransform` (`self.GetRandomPoint`)) "Undefined" "MultiplyWithRoot" null null))

(fn `GetRandomPoint`
  (returns (RandomPoint :type "Vector Structure"))
  (bind (_returnvalue_x _returnvalue_y) (`KismetMathLibrary.BreakVector` (`BoxComponent.GetScaledBoxExtent` (`self.SpawnZone`))))
  (return (`KismetMathLibrary.RandomPointInBoundingBox` (`self.K2_GetActorLocation`) (`KismetMathLibrary.MakeVector` _returnvalue_x _returnvalue_y))))

(fn `UserConstructionScript`
  (`parent.UserConstructionScript`)
  (`BoxComponent.SetBoxExtent` (`self.SpawnZone`) (`KismetMathLibrary.MakeVector` (/ (`self.ZoneHeight`) 2.0) (/ (`self.ZoneWidth`) 2.0) 100.0) true))