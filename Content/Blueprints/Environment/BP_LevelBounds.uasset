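; Level bounds actor that wraps BP_BaseCharacter actors to the far side of the play area when they overlap an edge box.
; Construction script sizes four edge boxes from Width, Height and Depth and offsets them, though BoundsBottom uses Height squared, not negative Height.
; Overlaps mirror the closest collision point through the actor's origin in XY, nudged inward by the character's box extent.
; The swept move keeps Z; OppositeBox is unused.
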(event `self.BoundsTop.OnComponentBeginOverlap`
  (params (OverlappedComponent :type "PrimitiveComponent Object Reference") (OtherActor :type "Actor Object Reference") (OtherComp :type "PrimitiveComponent Object Reference") (OtherBodyIndex :type Integer) (bFromSweep :type Boolean) (SweepResult :type "HitResult Structure (by ref)"))
  (`self.TeleportActor` OtherActor OverlappedComponent (`self.BoundsBottom`)))

(event `self.BoundsBottom.OnComponentBeginOverlap`
  (params (OverlappedComponent :type "PrimitiveComponent Object Reference") (OtherActor :type "Actor Object Reference") (OtherComp :type "PrimitiveComponent Object Reference") (OtherBodyIndex :type Integer) (bFromSweep :type Boolean) (SweepResult :type "HitResult Structure (by ref)"))
  (`self.TeleportActor` OtherActor OverlappedComponent (`self.BoundsTop`)))

(event `self.BoundsRight.OnComponentBeginOverlap`
  (params (OverlappedComponent :type "PrimitiveComponent Object Reference") (OtherActor :type "Actor Object Reference") (OtherComp :type "PrimitiveComponent Object Reference") (OtherBodyIndex :type Integer) (bFromSweep :type Boolean) (SweepResult :type "HitResult Structure (by ref)"))
  (`self.TeleportActor` OtherActor OverlappedComponent (`self.BoundsLeft`)))

(event `self.BoundsLeft.OnComponentBeginOverlap`
  (params (OverlappedComponent :type "PrimitiveComponent Object Reference") (OtherActor :type "Actor Object Reference") (OtherComp :type "PrimitiveComponent Object Reference") (OtherBodyIndex :type Integer) (bFromSweep :type Boolean) (SweepResult :type "HitResult Structure (by ref)"))
  (`self.TeleportActor` OtherActor OverlappedComponent (`self.BoundsRight`)))

(fn `GetExitPoint`
  (params (OtherActor :type "Actor Object Reference") (Box :type "PrimitiveComponent Object Reference"))
  (returns (ExitPoint :type "Vector Structure"))
  (return (`PrimitiveComponent.GetClosestPointOnCollision` Box (`self.K2_GetActorLocation` OtherActor) "None")))

(fn `GetOppositeLocation`
  (params (OtherActor :type "Actor Object Reference") (SurfacePoint :type "Vector Structure"))
  (returns (Location :type "Vector Structure"))
  (bind (_returnvalue_x _returnvalue_y _returnvalue_z) (`KismetMathLibrary.BreakVector` (`self.K2_GetActorLocation` OtherActor)))
  (bind _returnvalue (`self.K2_GetActorLocation`))
  (bind _returnvalue_2 (- SurfacePoint _returnvalue))
  (bind _asbp_base_character (cast `/Game/Blueprints/Character/BP_BaseCharacter` OtherActor))
  (bind (_returnvalue_x_2 _returnvalue_y_2) (`KismetMathLibrary.BreakVector` (+ (* _returnvalue_2 -1.0) _returnvalue (* (`KismetMathLibrary.Normal` _returnvalue_2) (`KismetMathLibrary.VSizeXY` (`BoxComponent.GetScaledBoxExtent` (`/Game/Blueprints/Character/BP_BaseCharacter.CollisionBox` _asbp_base_character)))))))
  (return (`KismetMathLibrary.MakeVector` _returnvalue_x_2 _returnvalue_y_2 _returnvalue_z)))

(fn `TeleportActor`
  (params (OtherActor :type "Actor Object Reference") (Box :type "PrimitiveComponent Object Reference") (OppositeBox :type "PrimitiveComponent Object Reference"))
  (locals (OldVelocity :type "Vector Structure"))
  (cast `/Game/Blueprints/Character/BP_BaseCharacter` OtherActor)
  (bind _exitpoint (`self.GetExitPoint` OtherActor Box))
  (bind _location (`self.GetOppositeLocation` OtherActor _exitpoint))
  (`self.K2_SetActorLocation` OtherActor _location true false))

(fn `UserConstructionScript`
  (bind _height (`self.Height`))
  (bind _width (`self.Width`))
  (`|ExecutionSequence`
    (:`then_0`
      ;[1 1 1] Set box extents
      (`BoxComponent.SetBoxExtent` (`self.BoundsTop`) (`KismetMathLibrary.MakeVector` (/ (`self.Width`) 2.0) (/ (`self.Height`) 2.0) (/ (`self.Depth`) 2.0)) true)
      (`BoxComponent.SetBoxExtent` (`self.BoundsBottom`) (`KismetMathLibrary.MakeVector` (/ (`self.Width`) 2.0) (/ (`self.Height`) 2.0) (/ (`self.Depth`) 2.0)) true)
      (`BoxComponent.SetBoxExtent` (`self.BoundsLeft`) (`KismetMathLibrary.MakeVector` (/ (`self.Width`) 2.0) (/ (`self.Height`) 2.0) (/ (`self.Depth`) 2.0)) true)
      (`BoxComponent.SetBoxExtent` (`self.BoundsRight`) (`KismetMathLibrary.MakeVector` (/ (`self.Width`) 2.0) (/ (`self.Height`) 2.0) (/ (`self.Depth`) 2.0)) true))
    (:`then_1`
      (`SceneComponent.K2_AddRelativeLocation` (`self.BoundsTop`) (`KismetMathLibrary.MakeVector` 0.0 _height) false false)
      (`SceneComponent.K2_AddRelativeLocation` (`self.BoundsBottom`) (`KismetMathLibrary.MakeVector` 0.0 (* _height _height)) false false)
      (`SceneComponent.K2_AddRelativeLocation` (`self.BoundsRight`) (`KismetMathLibrary.MakeVector` _width) false false)
      (`SceneComponent.K2_AddRelativeLocation` (`self.BoundsLeft`) (`KismetMathLibrary.MakeVector` (* _width -1.0)) false false))))