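; BP_HealPickup is a pickup that restores health to the player who collects it.
; It overrides the inherited PickUp function, calls the parent version, then adds its own Health value to the player's Health, capped at the player's MaxHealth.
; All other behavior comes from the parent class, as the event graph holds only disabled default nodes and the construction script just calls the parent.
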(fn `PickUp`
  (params (Player :type "/Game/Blueprints/Character/Player/BP_Player Object Reference"))
  (`parent.PickUp` Player)
  (set `/Game/Blueprints/Character/BP_BaseCharacter.Health` (`KismetMathLibrary.FMin` (+ (`self.Health`) (`/Game/Blueprints/Character/BP_BaseCharacter.Health` Player)) (`/Game/Blueprints/Character/BP_BaseCharacter.MaxHealth` Player)) Player))

(fn `UserConstructionScript`
  (`parent.UserConstructionScript`))