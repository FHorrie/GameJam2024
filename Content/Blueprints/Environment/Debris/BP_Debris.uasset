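; BP_Debris is a drifting environmental debris actor that damages what it touches and awards score when the player shoots it.
; Construction picks a random mesh and scales damage by average actor scale; Tick moves it along Direction at Speed without sweeping.
; Capsule overlaps apply environmental point damage.
; Incoming point damage adds Score through BP_DroidGameMode for player instigators, calls an empty TakeDamage function and spawns a hit particle.
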(event `self.ReceivePointDamage`
  (params (Damage :type "Float (single-precision)") (DamageType :type "DamageType Object Reference") (HitLocation :type "Vector Structure") (HitNormal :type "Vector Structure") (HitComponent :type "PrimitiveComponent Object Reference") (BoneName :type Name) (ShotFromDirection :type "Vector Structure") (InstigatedBy :type "Controller Object Reference") (DamageCauser :type "Actor Object Reference") (HitInfo :type "HitResult Structure (by ref)"))
  (bind (_returnvalue_location _returnvalue_rotation _returnvalue_scale) (`KismetMathLibrary.BreakTransform` (`self.GetTransform` self)))
  (`|ExecutionSequence`
    (:`then_0`
      (`/Engine/EditorBlueprintResources/StandardMacros.IsValid` InstigatedBy
        (:`Is Valid`
          (cast `/Game/Blueprints/Character/Player/BP_Player` (`Controller.K2_GetPawn` InstigatedBy))
          (bind _asbp_droid_game_mode (cast `/Game/Blueprints/BP_DroidGameMode` (`GameplayStatics.GetGameMode`)))
          (`/Game/Blueprints/BP_DroidGameMode.AddScore` _asbp_droid_game_mode (`self.Score`)))))
    (:`then_1`
      (`self.TakeDamage` ShotFromDirection DamageType DamageCauser)
      (`/Engine/EditorBlueprintResources/StandardMacros.IsValid` self
        (:`Is Valid`
          (`GameplayStatics.SpawnEmitterAtLocation` "/Game/FXVarietyPack/Particles/P_ky_hit2.P_ky_hit2" _returnvalue_location _returnvalue_rotation _returnvalue_scale))))))

(event `self.Capsule.OnComponentBeginOverlap`
  (params (OverlappedComponent :type "PrimitiveComponent Object Reference") (OtherActor :type "Actor Object Reference") (OtherComp :type "PrimitiveComponent Object Reference") (OtherBodyIndex :type Integer) (bFromSweep :type Boolean) (SweepResult :type "HitResult Structure (by ref)"))
  (`self.Hit` OtherActor))

(event `self.ReceiveTick`
  (params (DeltaSeconds :type "Float (single-precision)"))
  (`self.UpdateLocation` DeltaSeconds))

(fn `AddScore`)

(fn `GetAverageScale`
  (returns (AverageScale :type "Float (double-precision)"))
  (bind (_returnvalue_x _returnvalue_y _returnvalue_z) (`KismetMathLibrary.BreakVector` (`self.GetActorScale3D`)))
  (return (/ (+ _returnvalue_x _returnvalue_y _returnvalue_z) 3.0)))

(fn `Hit`
  (params (`Hit Actor` :type "Actor Object Reference"))
  (`/Engine/EditorBlueprintResources/StandardMacros.IsValid` `Hit Actor`
    (:`Is Valid`
      (`GameplayStatics.ApplyPointDamage` `Hit Actor` (`self.InstanceDamage`) (- (`self.K2_GetActorLocation` `Hit Actor`) (`self.K2_GetActorLocation` self)) (`GameplayStatics.MakeHitResult` false true) null self "/Engine/EngineDamageTypes/DmgTypeBP_Environmental.DmgTypeBP_Environmental_C"))))

(fn `TakeDamage`
  (params (ShotFromDirection :type "Vector Structure") (DamageType :type "DamageType Object Reference") (DamageCauser :type "Actor Object Reference")))

(fn `UpdateLocation`
  (params (DeltaTime :type "Float (double-precision)"))
  (`self.K2_AddActorWorldOffset` (* DeltaTime (* (`self.Direction`) (`self.Speed`)))))

(fn `UserConstructionScript`
  (set `self.InstanceDamage` (* (`self.GetAverageScale`) (`self.BaseDamage`)))
  (`StaticMeshComponent.SetStaticMesh` (`self.Sphere`) (`KismetArrayLibrary.Array_Random` (`self.StaticMeshes`))))