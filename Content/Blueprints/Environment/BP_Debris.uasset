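; Moving debris hazard that travels along its Direction at Speed each tick, without sweeping.
; The construction script scales BaseDamage by average actor scale into InstanceDamage.
; On overlap, Hit calls ApplyPointDamage with that value, environmental damage type and direction toward the other actor, but sets no damaged actor.
; Any point damage received calls the empty TakeDamage stub, then destroys the debris.
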(event `self.ReceiveBeginPlay`
  (add `self.OnTakePointDamage` (delegate `OnTakePointDamage_Event`)))

(event `OnTakePointDamage_Event` :!signature `self.OnTakePointDamage`
  (params (DamagedActor :type "Actor Object Reference") (Damage :type "Float (single-precision)") (InstigatedBy :type "Controller Object Reference") (HitLocation :type "Vector Structure") (FHitComponent :type "PrimitiveComponent Object Reference") (BoneName :type Name) (ShotFromDirection :type "Vector Structure") (DamageType :type "DamageType Object Reference") (DamageCauser :type "Actor Object Reference"))
  (`self.TakeDamage` ShotFromDirection DamageType DamageCauser)
  (`self.K2_DestroyActor`))

(event `self.ReceiveActorBeginOverlap`
  (params (OtherActor :type "Actor Object Reference"))
  (`self.Hit` OtherActor))

(event `self.ReceiveTick`
  (params (DeltaSeconds :type "Float (single-precision)"))
  (`self.UpdateLocation` DeltaSeconds))

(fn `GetAverageScale`
  (returns (AverageScale :type "Float (double-precision)"))
  (bind (_returnvalue_x _returnvalue_y _returnvalue_z) (`KismetMathLibrary.BreakVector` (`self.GetActorScale3D`)))
  (return (/ (+ _returnvalue_x _returnvalue_y _returnvalue_z) 3.0)))

(fn `Hit`
  (params (`Hit Actor` :type "Actor Object Reference"))
  (`GameplayStatics.ApplyPointDamage` null (`self.InstanceDamage`) (- (`self.K2_GetActorLocation` `Hit Actor`) (`self.K2_GetActorLocation` self)) (`GameplayStatics.MakeHitResult` false true) null self "/Engine/EngineDamageTypes/DmgTypeBP_Environmental.DmgTypeBP_Environmental_C"))

(fn `TakeDamage`
  (params (ShotFromDirection :type "Vector Structure") (DamageType :type "DamageType Object Reference") (DamageCauser :type "Actor Object Reference")))

(fn `UpdateLocation`
  (params (DeltaTime :type "Float (double-precision)"))
  (`self.K2_AddActorWorldOffset` (* DeltaTime (* (`self.Direction`) (`self.Speed`)))))

(fn `UserConstructionScript`
  (set `self.InstanceDamage` (* (`self.GetAverageScale`) (`self.BaseDamage`))))