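; Player controller that adds the player input mapping context and drives the controlled pawn's movement and yaw rotation.
; Move input blends the pawn's forward vector with its velocity direction into a normalized movement direction, while rotate input adds yaw scaled by RotationSpeed.
; A LookAtMouse function lerps control rotation toward a traced cursor hit point, but nothing in this Blueprint calls it.
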(event `self.ReceiveBeginPlay`
  (bind _returnvalue (subsystem `EnhancedInputLocalPlayerSubsystem`))
  (`/Engine/EditorBlueprintResources/StandardMacros.IsValid` _returnvalue
    (:`Is Valid`
      (`EnhancedInputSubsystemInterface.AddMappingContext` _returnvalue "/Game/Blueprints/Input/IMC_PlayerInput.IMC_PlayerInput" 0 (struct)))))

(event `self.ReceiveTick`
  (params (DeltaSeconds :type "Float (single-precision)")))

(event `EnhancedInput|/Game/Blueprints/Input/Controls/IA_Move`
  (params (ActionValue :type "Float (double-precision)") (ElapsedSeconds :type "Float (double-precision)") (TriggeredSeconds :type "Float (double-precision)") (InputAction :type "InputAction Object Reference" :default "/Game/Blueprints/Input/Controls/IA_Move.IA_Move"))
  (bind _returnvalue (`self.K2_GetPawn`))
  (:`Triggered`
    (`Pawn.AddMovementInput` _returnvalue (`KismetMathLibrary.Normal` (* (+ (`self.GetActorForwardVector` _returnvalue) (`KismetMathLibrary.Normal` (`self.GetVelocity` _returnvalue))) ActionValue)) 1.0 true)))

(event `EnhancedInput|/Game/Blueprints/Input/Controls/IA_Rotate`
  (params (ActionValue :type "Float (double-precision)") (ElapsedSeconds :type "Float (double-precision)") (TriggeredSeconds :type "Float (double-precision)") (InputAction :type "InputAction Object Reference" :default "/Game/Blueprints/Input/Controls/IA_Rotate.IA_Rotate"))
  (:`Triggered`
    (`self.AddYawInput` (* (`self.RotationSpeed`) ActionValue))))

(fn `LookAtMouse`
  (params (DeltaTime :type "Float (double-precision)"))
  (bind (_worldlocation _worlddirection) (`self.DeprojectMousePositionToWorld`))
  (bind _outhit (`KismetSystemLibrary.LineTraceSingle` _worldlocation (+ _worldlocation (* _worlddirection 10000.0)) "TraceTypeQuery1"))
  (`self.SetControlRotation` (`KismetMathLibrary.RLerp` (`self.GetDesiredRotation`) (`KismetMathLibrary.MakeRotFromX` (- (`.Location` (`GameplayStatics.BreakHitResult` _outhit)) (`self.K2_GetActorLocation` (`self.K2_GetPawn`)))) (* DeltaTime (`self.LerpIntensity`)) true)))

(fn `UserConstructionScript`)